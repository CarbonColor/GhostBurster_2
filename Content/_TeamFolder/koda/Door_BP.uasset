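; Door Blueprint that swings its Door component open when a separate opener actor signals it.
; On BeginPlay it looks up that actor by the class of its Open variable, stores it there and binds PlayerCom to its OpenToDoor event.
; PlayerCom calls OpenDoor, which plays the TM_Door timeline to interpolate the door's relative yaw through a quarter turn.
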(event Custom|OpenDoor
  (bind _新規track_0 (Timeline|TM_Door Play)
    (:Update
      (Transformation|SetRelativeRotation (Variables|Default|GetDoor) (Math|Rotator|MakeRotator 0.0 0.0 (Math|Float|Lerp 0.0 -9e+01 _新規track_0)) false false))))

(event Custom|PlayerCom
  (CallFunction|OpenDoor))

(event EventBeginPlay
  (bind _returnvalue (Actor|GetActorOfClass (Utilities|GetClass (Variables|Default|GetOpen))))
  (bind _output_get (Variables|Default|SetOpen _returnvalue))
  (EventDispatchers|BindEventtoOpenDoor _output_get (delegate Custom|PlayerCom)))

(event Collision|EventActorBeginOverlap
  (params (OtherActor :type Actor%20Object%20Reference)))

(event EventTick
  (params (DeltaSeconds :type Float%20%28single-precision%29)))

(fn ConstructionScript)
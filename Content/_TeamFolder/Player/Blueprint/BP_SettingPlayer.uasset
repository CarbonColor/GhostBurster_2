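; BP_SettingPlayer is the player for device setup, reading a finger-sensor device over a serial COM port for calibration.
; BeginPlay opens the port number stored in PlayerScoreInstance, and EndPlay flushes and closes it.
; Each Tick parses comma-separated readings into the Finger array and shows the raw string on the calibration widget.
; EventNumber then selects the normal, fox or gun pose check while measuring, or the used-item check regardless.
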(event EventBeginPlay
  ;[1 1 1] ポート番号とボーレートの設定
  (bind _asplayer_score_instance (Utilities|Casting|CastToPlayerScoreInstance (Game|GetGameInstance))
    (:then
      ;[1 1 1] デバイスの接続処理
      (bind (_bopened _returnvalue) (Class|SerialCom|OpenComPort (Variables|/Script/GhostBurster.PlayerScoreInstance|GetDevicePortNumber _asplayer_score_instance) (Variables|Default|GetBoadRate)))
      (if _bopened
        (Variables|Default|SetDevice _returnvalue)
        (else
          (Development|PrintString "未接続" true true "(R=1.000000,G=0.000000,B=0.000000,A=1.000000)" 1e+01))))
    (:CastFailed
      (Development|PrintString "Not Player Score Instance" true true "(R=1.000000,G=0.000000,B=0.000000,A=1.000000)" 3.0))))

(event EventTick
  (params (DeltaSeconds :type Float%20%28single-precision%29))
  (bind _finger (Variables|Default|GetFinger))
  (bind _device (Variables|Default|GetDevice))
  (Utilities|IsValid _device
    (:Is%20Valid
      (bind (_bsuccess _returnvalue) (Class|SerialCom|ReadString _device))
      (if _bsuccess
        (bind _asui_device_setting_finger (Utilities|Casting|CastToUI_DeviceSetting_Finger (UserInterface|GetWidget (Variables|Default|GetCalibrationWidgetComponent))))
        (Default|SettingText _asui_device_setting_finger (Utilities|Text|ToText(String) _returnvalue))
        (for (_array_element _array_index) (Utilities|String|ParseIntoArray _returnvalue ",")
          (Utilities|Array|SetArrayElem (Variables|Default|GetFinger) _array_index (Math|Conversions|ToInteger(Byte) _array_element)))
        (switch int (Variables|Default|GetEventNumber)
          (:2
            (if (Variables|Default|GetbIsMeasuring)
              (Class|SettingPlayer|CheckNormalFinger _finger)))
          (:4
            (if (Variables|Default|GetbIsMeasuring)
              (Class|SettingPlayer|CheckFoxFinger _finger)))
          (:6
            (if (Variables|Default|GetbIsMeasuring)
              (Class|SettingPlayer|CheckGunFinger _finger)))
          (:7
            (Class|SettingPlayer|CheckUsedItem (Variables|Default|GetFinger))))))))

(event EventEndPlay
  (params (EndPlayReason :type EEndPlayReason%20Enum :default "Destroyed"))
  ;[1 1 1] ゲーム終了時にCOMポートを閉じる
  (Utilities|IsValid (Variables|Default|GetDevice)
    (:Is%20Valid
      (if (Class|SerialCom|IsOpened (Variables|Default|GetDevice))
        (Class|SerialCom|Flush (Variables|Default|GetDevice))
        (Class|SerialCom|Close (Variables|Default|GetDevice))
        (Variables|Default|SetDevice 0)
        (else
          (Variables|Default|SetDevice 0))))))

(fn ConstructionScript)
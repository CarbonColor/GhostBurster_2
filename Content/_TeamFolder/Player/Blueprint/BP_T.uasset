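; BP_T is a treasure chest that opens once when the VR player's LightCollision overlaps its box, then grants an item to the player.
; Chained timelines slide and rotate the lid, spawn a BP_Item offset by the chest's Direction setting and move it vertically.
; After a short delay, another timeline fades the item through its Opacity material parameter, then calls AddItem on the player and destroys it.
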(event OnComponentBeginOverlap(Box)
  (params (OverlappedComponent :type Primitive%20Component%20Object%20Reference) (OtherActor :type Actor%20Object%20Reference) (OtherComp :type Primitive%20Component%20Object%20Reference) (OtherBodyIndex :type Integer) (bFromSweep :type Boolean) (SweepResult :type Hit%20Result%20Structure%20%28by%20ref%29))
  (bind _coverlocation (Variables|Default|GetCoverLocation))
  (if (== OtherComp (Variables|/Script/GhostBurster.VRPlayerCharacter|GetLightCollision (Variables|Default|GetPlayer)))
    (if (not (Variables|Default|GetIsOpened))
      (Variables|Default|SetIsOpened true)
      (Audio|PlaySoundatLocation "/Game/_TeamFolder/Sound/SE/SE_OpenTreasure_Cue.SE_OpenTreasure_Cue" (Transformation|GetWorldLocation (Variables|Default|GetDefaultSceneRoot)) "0, 0, 0" 1.0 1.0 0.0 0 0 0 0)
      ;[1 1 1] 蓋を開ける処理
      (bind (_direction _coverrotation _coverlocationy _coverlocationz) (Timeline|OpenCover Play)
        (:Update
          (Transformation|SetRelativeTransform (Variables|Default|GetTreasureCover) (Math|Transform|MakeTransform (Math|Vector|MakeVector (.x _coverlocation) (+ (.y _coverlocation) _coverlocationy) (+ (.z _coverlocation) _coverlocationz)) (Math|Rotator|MakeRotator (Math|Float|Lerp 0.0 -9e+01 _coverrotation) 0.0 0.0) (.scale (Transformation|GetRelativeTransform (Variables|Default|GetTreasureCover)))) false false))
        (:Finished
          ;[1 1 1] アイテムの出現処理
          (bind _returnvalue (Game|SpawnActorfromClass "/Game/_TeamFolder/Player/Blueprint/BP_Item.BP_Item_C" (Math|Transform|MakeTransform (+ (.location (Transformation|GetRelativeTransform (Variables|Default|GetDefaultSceneRoot))) (Variables|Default|GetItemOffset)) "0, 0, 0" (Variables|Default|GetItemScale)) "Undefined" "MultiplyWithRoot" 0 0))
          (bind _output_get (Variables|Default|SetItem _returnvalue))
          (Variables|Default|SetItemLocation (.location (Transformation|GetActorTransform _output_get)))
          ;[1 1 1] アイテムの移動処理
          (bind _itemlocation (Timeline|ItemMotion Play)
            (:Update
              (Transformation|SetActorTransform (Variables|Default|GetItem) (Math|Transform|MakeTransform (Math|Vector|MakeVector (.x (Variables|Default|GetItemLocation)) (.y (Variables|Default|GetItemLocation)) (+ (.z (Variables|Default|GetItemLocation)) _itemlocation)) "0, 0, 0" (.scale (Transformation|GetActorTransform _output_get)))))
            (:Finished
              ;[1 1 1] アイテムが消える処理
              (Utilities|FlowControl|Delay 1.0)
              (Audio|PlaySoundatLocation "/Game/_TeamFolder/Sound/SE/SE_GetItem_Cue.SE_GetItem_Cue" (Transformation|GetWorldLocation (Variables|Default|GetDefaultSceneRoot)) "0, 0, 0" 1.0 1.0 0.0 0 0 0 0)
              (bind _fadeoutitem (Timeline|DestroyItem Play)
                (:Update
                  (Rendering|Material|SetScalarParameterValueonMaterials (Variables|/Game/_TeamFolder/Player/Blueprint/BP_Item.BP_Item_C|GetTest (Variables|Default|GetItem)) "Opacity" _fadeoutitem))
                (:Finished
                  (Class|VRPlayerCharacter|AddItem (Variables|Default|GetPlayer))
                  (Actor|DestroyActor (Variables|Default|GetItem)))))))))))

(event EventBeginPlay
  ;[1 1 1] 初期化
  (bind _returnvalue (Actor|GetActorOfClass "/Script/GhostBurster.VRPlayerCharacter"))
  (Variables|Default|SetPlayer _returnvalue)
  (Variables|Default|SetIsOpened false)
  ;[1 1 1] 蓋の座標を保存
  (Variables|Default|SetCoverLocation (.location (Transformation|GetRelativeTransform (Variables|Default|GetTreasureCover))))
  ;[1 1 1] 宝箱の向きによってアイテムの出現座標のOffsetを変更
  (switch Utilities|FlowControl|Switch|SwitchonTreasureBoxDirection (Variables|Default|GetDirection)
    (:NewEnumerator2
      (Variables|Default|SetItemOffset "0.000000,35.000000,0.000000"))
    (:NewEnumerator1
      (Variables|Default|SetItemOffset "-35.000000,0.000000,0.000000"))
    (:NewEnumerator3
      (Variables|Default|SetItemOffset "0.000000,-35.000000,0.000000"))
    (:NewEnumerator0
      (Variables|Default|SetItemOffset "35.000000,0.000000,0.000000"))))

(fn ConstructionScript)
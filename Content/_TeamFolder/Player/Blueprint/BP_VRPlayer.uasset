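; VR player Blueprint that links a finger-bend sensing, vibrating glove to the game over a serial COM port.
; BeginPlay opens the port number stored in PlayerScoreInstance, and EndPlay flushes and closes it.
; Tick parses comma-separated readings into the finger sensor array and passes it to CheckUsedItem.
; Two events write integer codes back to the glove to trigger item-use and damage vibration.
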(event EventBeginPlay
  ;[1 1 1] ポート番号とボーレートの設定
  (bind _asplayer_score_instance (Utilities|Casting|CastToPlayerScoreInstance (Game|GetGameInstance))
    (:then
      ;[1 1 1] デバイスの接続処理
      (bind (_bopened _returnvalue) (Class|SerialCom|OpenComPort (Variables|/Script/GhostBurster.PlayerScoreInstance|GetDevicePortNumber _asplayer_score_instance) (Variables|Default|GetBuadRate)))
      (if _bopened
        (Variables|Default|SetGloveDevice _returnvalue)
        (else
          (Development|PrintString "未接続" true true "(R=1.000000,G=0.000000,B=0.000000,A=1.000000)" 1e+01))))
    (:CastFailed
      (Development|PrintString "Not Player Score Instance" true true "(R=1.000000,G=0.000000,B=0.000000,A=1.000000)" 3.0))))

(event EventGloveDeviceVibrationUseItem
  (bind _exportnum_useitem (Variables|Default|GetExportNum_UseItem))
  (bind _glovedevice (Variables|Default|GetGloveDevice))
  (Utilities|IsValid _glovedevice
    (:Is%20Valid
      (bind _returnvalue (Class|SerialCom|WriteInt _glovedevice _exportnum_useitem))
      (if _returnvalue
        (Development|PrintString (Utilities|String|ToString(Integer) _exportnum_useitem) true true "(R=0.206075,G=1.000000,B=0.746630,A=1.000000)" 3.0)))))

(event EventTick
  (params (DeltaSeconds :type Float%20%28single-precision%29))
  (bind _glovedevice (Variables|Default|GetGloveDevice))
  ;[1 1 1] デバイスから指の曲げ具合を受け取り、配列に入れる処理
  (Utilities|IsValid _glovedevice
    (:Is%20Valid
      (bind (_bsuccess _returnvalue) (Class|SerialCom|ReadString _glovedevice))
      (if _bsuccess
        (for (_array_element _array_index) (Utilities|String|ParseIntoArray _returnvalue ",")
          (Utilities|Array|SetArrayElem (Variables|Default|GetFIngerSensor) _array_index (Math|Conversions|ToInteger(Byte) _array_element))
          (Development|PrintString _returnvalue false true "(R=1.000000,G=1.000000,B=1.000000,A=1.000000)" 0.02))
        (Class|VRPlayerCharacter|CheckUsedItem (Variables|Default|GetFIngerSensor))))))

(event EventEndPlay
  (params (EndPlayReason :type EEndPlayReason%20Enum :default "Destroyed"))
  ;[1 1 1] ゲーム終了時にCOMポートを閉じる
  (Utilities|IsValid (Variables|Default|GetGloveDevice)
    (:Is%20Valid
      (if (Class|SerialCom|IsOpened (Variables|Default|GetGloveDevice))
        (Class|SerialCom|Flush (Variables|Default|GetGloveDevice))
        (Class|SerialCom|Close (Variables|Default|GetGloveDevice))
        (Variables|Default|SetGloveDevice 0)
        (else
          (Variables|Default|SetGloveDevice 0))))))

(event EventGloveDeviceVibrationDamage
  (bind _exportnum_damage (Variables|Default|GetExportNum_Damage))
  (bind _glovedevice (Variables|Default|GetGloveDevice))
  (Utilities|IsValid _glovedevice
    (:Is%20Valid
      (bind _returnvalue (Class|SerialCom|WriteInt _glovedevice _exportnum_damage))
      (if _returnvalue
        (Development|PrintString (Utilities|String|ToString(Integer) _exportnum_damage) true true "(R=0.206075,G=1.000000,B=0.746630,A=1.000000)" 3.0)))))

(fn ConstructionScript)
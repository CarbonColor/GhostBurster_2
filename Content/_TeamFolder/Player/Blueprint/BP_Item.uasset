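; BP_Item is an item pickup actor that plays a collection effect on BeginPlay and credits the item to the VR player.
; A timeline raises it from its spawn position along Z.
; After a one-second delay, it plays the pickup sound while a second timeline drives the Niagara Opacity parameter to fade it out.
; When the fade finishes, it calls AddItem on the VRPlayerCharacter and destroys itself.
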(event EventBeginPlay
  ;[1 1 1] プレイヤー取得
  (bind _returnvalue (Actor|GetActorOfClass "/Script/GhostBurster.VRPlayerCharacter"))
  (Variables|Default|SetPlayer _returnvalue)
  ;[1 1 1] マテリアルを取得して不透明にする
  (Niagara|SetNiagaraVariable(Float) (Variables|Default|GetNiagaraComponent) "Opacity" 1.0)
  ;[1 1 1] 初期座標を保存
  (Variables|Default|SetInitialLocation (Transformation|GetWorldLocation (Variables|Default|GetDefaultSceneRoot)))
  ;[1 1 1] 真上に動かす処理
  (bind _itemlocation (Timeline|MoveTimeline Play)
    (:Update
      (Transformation|SetActorTransform (Math|Transform|MakeTransform (Math|Vector|MakeVector (.x (Variables|Default|GetInitialLocation)) (.y (Variables|Default|GetInitialLocation)) (+ (.z (Variables|Default|GetInitialLocation)) _itemlocation)) "0, 0, 0" (Transformation|GetWorldScale (Variables|Default|GetDefaultSceneRoot)))))
    (:Finished
      ;[1 1 1] 徐々に透明にする処理
      (Utilities|FlowControl|Delay 1.0)
      (Audio|PlaySoundatLocation "/Game/_TeamFolder/Sound/SE/SE_GetItem_Cue.SE_GetItem_Cue" (Transformation|GetWorldLocation (Variables|Default|GetDefaultSceneRoot)) "0, 0, 0" 1.0 1.0 0.0 0 0 0 0)
      (bind _fadeoutitem (Timeline|FadeOutTimeline Play)
        (:Update
          (Niagara|SetNiagaraVariable(Float) (Variables|Default|GetNiagaraComponent) "Opacity" _fadeoutitem))
        (:Finished
          ;[1 1 1] プレイヤーにアイテムを加算して自信を消す
          (Class|VRPlayerCharacter|AddItem (Variables|Default|GetPlayer))
          (Actor|DestroyActor))))))

(fn ConstructionScript)
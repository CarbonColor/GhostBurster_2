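; Double-door Blueprint that swings open with a sound when the VR player enters its trigger box, and runs a close animation on exit.
; BeginPlay caches the player and both leaves' relative locations; overlaps count only for the player's PlayerCollision.
; Separate open and close timelines lerp yaw, with opening also offsetting each leaf's position.
; The close timeline writes both transforms to the same leaf, leaving the other untouched.
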(event OnComponentEndOverlap(Box)
  (params (OverlappedComponent :type Primitive%20Component%20Object%20Reference) (OtherActor :type Actor%20Object%20Reference) (OtherComp :type Primitive%20Component%20Object%20Reference) (OtherBodyIndex :type Integer))
  (if (== OtherComp (Variables|/Script/GhostBurster.VRPlayerCharacter|GetPlayerCollision (Variables|Default|Getplayer)))
    (CallFunction|CloseDoor)))

(event OnComponentBeginOverlap(Box)
  (params (OverlappedComponent :type Primitive%20Component%20Object%20Reference) (OtherActor :type Actor%20Object%20Reference) (OtherComp :type Primitive%20Component%20Object%20Reference) (OtherBodyIndex :type Integer) (bFromSweep :type Boolean) (SweepResult :type Hit%20Result%20Structure%20%28by%20ref%29))
  (if (== OtherComp (Variables|/Script/GhostBurster.VRPlayerCharacter|GetPlayerCollision (Variables|Default|Getplayer)))
    (CallFunction|OpenDoor)))

(event Custom|OpenDoor
  (bind _door_r (Variables|Default|Getdoor_R))
  (bind _door (Variables|Default|Getdoor))
  (Audio|PlaySoundatLocation "/Game/_TeamFolder/Sound/SE/SE_OpenDoor.SE_OpenDoor" (Transformation|GetWorldLocation (Variables|Default|GetDefaultSceneRoot)) "0, 0, 0" 1.0 1.0 0.0 0 0 0 0)
  (bind (_direction _新規track_0 _新規track_1) (Timeline|TM_Door Play)
    (:Update
      (Transformation|SetRelativeTransform (Variables|Default|GetVR_door_A_VR_door_R) (Math|Transform|MakeTransform (Math|Vector|MakeVector (+ (.x _door_r) 1e+01) (+ (.y _door_r) -1e+01) (.z _door_r)) (Math|Rotator|MakeRotator 0.0 0.0 (Math|Float|Lerp 0.0 9e+01 _新規track_0)) (.scale (Transformation|GetRelativeTransform (Variables|Default|GetVR_door_A_VR_door_R)))) false false)
      (Transformation|SetRelativeTransform (Variables|Default|GetVR_door_A_VR_door_R1) (Math|Transform|MakeTransform (Math|Vector|MakeVector (+ (.x _door) -1e+01) (+ (.y _door) -25.0) (.z _door)) (Math|Rotator|MakeRotator 0.0 0.0 (Math|Float|Lerp 1.8e+02 9e+01 _新規track_1)) (.scale (Transformation|GetRelativeTransform (Variables|Default|GetVR_door_A_VR_door_R1)))) false false))))

(event Custom|CloseDoor
  (bind _door_r (Variables|Default|Getdoor_R))
  (bind _door_r_2 (Variables|Default|Getdoor_R))
  (bind (_direction _新規track_0 _新規track_1) (Timeline|タイムライン Play)
    (:Update
      (Transformation|SetRelativeTransform (Variables|Default|GetVR_door_A_VR_door_R) (Math|Transform|MakeTransform (Math|Vector|MakeVector (.x _door_r) (.y _door_r) (.z _door_r)) (Math|Rotator|MakeRotator 0.0 0.0 (Math|Float|Lerp 0.0 -9e+01 _新規track_0)) (.scale (Transformation|GetRelativeTransform (Variables|Default|GetVR_door_A_VR_door_R)))) false false)
      (Transformation|SetRelativeTransform (Variables|Default|GetVR_door_A_VR_door_R) (Math|Transform|MakeTransform (Math|Vector|MakeVector (.x _door_r_2) (.y _door_r_2) (.z _door_r_2)) (Math|Rotator|MakeRotator 0.0 0.0 (Math|Float|Lerp 9e+01 1.8e+02 _新規track_1)) "1.000000,1.000000,1.000000") false false))))

(event EventBeginPlay
  (bind _returnvalue (Actor|GetActorOfClass "/Script/GhostBurster.VRPlayerCharacter"))
  (Variables|Default|Setplayer _returnvalue)
  (Variables|Default|Setdoor_R (.location (Transformation|GetRelativeTransform (Variables|Default|GetVR_door_A_VR_door_R))))
  (Variables|Default|Setdoor (.location (Transformation|GetRelativeTransform (Variables|Default|GetVR_door_A_VR_door_R1)))))

(fn ConstructionScript)
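; Trigger actor that manages the start and end of a VR run along the player's spline path.
; On BeginPlay it finds the player and PlayerSplinePath, then after a delay records the start time in PlayerScoreInstance and starts spline movement.
; When the player's collision enters the box, it records the end time, plays a fade sound and opens the Ending level.
; A Debug event stops movement and runs the same ending.
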(event OnComponentBeginOverlap(Box)
  (params (OverlappedComponent :type Primitive%20Component%20Object%20Reference) (OtherActor :type Actor%20Object%20Reference) (OtherComp :type Primitive%20Component%20Object%20Reference) (OtherBodyIndex :type Integer) (bFromSweep :type Boolean) (SweepResult :type Hit%20Result%20Structure%20%28by%20ref%29))
  (if (== OtherComp (Variables|/Script/GhostBurster.VRPlayerCharacter|GetPlayerCollision (Variables|Default|GetPlayer)))
    (Class|PlayerScoreInstance|SetGameEndTime (Variables|Default|GetGameInstance))
    (Utilities|FlowControl|Delay 3.0)
    (Audio|PlaySound2D "/Game/_TeamFolder/Sound/SE/SE_GameEndFade_Cue.SE_GameEndFade_Cue" 1.0 1.0 0.0 0 0)
    (Utilities|FlowControl|Delay 3.0)
    (Game|OpenLevel(byName) "Ending")))

(event Custom|Debug
  (Class|PlayerSplinePath|StopMovement (Variables|Default|GetSpline))
  (Class|PlayerScoreInstance|SetGameEndTime (Variables|Default|GetGameInstance))
  (Utilities|FlowControl|Delay 3.0)
  (Audio|PlaySound2D "/Game/_TeamFolder/Sound/SE/SE_GameEndFade_Cue.SE_GameEndFade_Cue" 1.0 1.0 0.0 0 0)
  (Utilities|FlowControl|Delay 3.0)
  (Game|OpenLevel(byName) "Ending"))

(event EventBeginPlay
  ;[1 1 1] プレイヤーを取得
  (bind _returnvalue (Actor|GetActorOfClass "/Script/GhostBurster.VRPlayerCharacter"))
  (Variables|Default|SetPlayer _returnvalue)
  ;[1 1 1] プレイヤーのルートを取得
  (bind _returnvalue_2 (Actor|GetActorOfClass "/Script/GhostBurster.PlayerSplinePath"))
  (Variables|Default|SetSpline _returnvalue_2)
  ;[1 1 1] 3秒後にゲームスタート
  (Utilities|FlowControl|Delay 3.0)
  (bind _asplayer_score_instance (Utilities|Casting|CastToPlayerScoreInstance (Game|GetGameInstance)))
  (bind _output_get (Variables|Default|SetGameInstance _asplayer_score_instance))
  (Class|PlayerScoreInstance|SetGameStartTime _output_get)
  (Class|PlayerSplinePath|StartMovement (Variables|Default|GetSpline)))

(fn ConstructionScript)
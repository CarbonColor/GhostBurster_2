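; Double boss-room door that opens when the VR player's collision enters its trigger Box and closes when it leaves.
; BeginPlay caches the player and both leaves' relative locations.
; Separate open and close Timelines lerp leaf yaw from zero, with opposite target signs between opening and closing.
; Position is not interpolated: opening sets fixed offsets from the cached locations, and closing restores them.
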(event OnComponentBeginOverlap(Box)
  (params (OverlappedComponent :type Primitive%20Component%20Object%20Reference) (OtherActor :type Actor%20Object%20Reference) (OtherComp :type Primitive%20Component%20Object%20Reference) (OtherBodyIndex :type Integer) (bFromSweep :type Boolean) (SweepResult :type Hit%20Result%20Structure%20%28by%20ref%29))
  (if (== OtherComp (Variables|/Script/GhostBurster.VRPlayerCharacter|GetPlayerCollision (Variables|Default|Getplayer)))
    (CallFunction|OpenDoor)))

(event OnComponentEndOverlap(Box)
  (params (OverlappedComponent :type Primitive%20Component%20Object%20Reference) (OtherActor :type Actor%20Object%20Reference) (OtherComp :type Primitive%20Component%20Object%20Reference) (OtherBodyIndex :type Integer))
  (if (== OtherComp (Variables|/Script/GhostBurster.VRPlayerCharacter|GetPlayerCollision (Variables|Default|Getplayer)))
    (CallFunction|CloseDoor)))

(event Custom|OpenDoor
  (bind _door_r (Variables|Default|Getdoor_R))
  (bind _door_l (Variables|Default|Getdoor_L))
  (bind (_direction _新規track_0 _新規track_1) (Timeline|タイムライン Play)
    (:Update
      (Transformation|SetRelativeTransform (Variables|Default|GetVR_door_A_VR_door_R) (Math|Transform|MakeTransform (Math|Vector|MakeVector (+ (.x _door_r) -6e+01) (+ (.y _door_r) 6e+01) (.z _door_r)) (Math|Rotator|MakeRotator 0.0 0.0 (Math|Float|Lerp 0.0 -9e+01 _新規track_0)) (.scale (Transformation|GetRelativeTransform (Variables|Default|GetVR_door_A_VR_door_R)))) false false)
      (Transformation|SetRelativeTransform (Variables|Default|GetVR_door_A_VR_door_L) (Math|Transform|MakeTransform (Math|Vector|MakeVector (+ (.x _door_l) 6e+01) (+ (.y _door_l) 6e+01) (.z _door_l)) (Math|Rotator|MakeRotator 0.0 0.0 (Math|Float|Lerp 0.0 9e+01 _新規track_1)) (.scale (Transformation|GetRelativeTransform (Variables|Default|GetVR_door_A_VR_door_L)))) false false))))

(event Custom|CloseDoor
  (bind _door_l (Variables|Default|Getdoor_L))
  (bind _door_r (Variables|Default|Getdoor_R))
  (bind (_direction _新規track_0 _新規track_1) (Timeline|タイムライン_0 Play)
    (:Update
      (Transformation|SetRelativeTransform (Variables|Default|GetVR_door_A_VR_door_R) (Math|Transform|MakeTransform (Math|Vector|MakeVector (.x _door_r) (.y _door_r) (.z _door_r)) (Math|Rotator|MakeRotator 0.0 0.0 (Math|Float|Lerp 0.0 9e+01 _新規track_0)) (.scale (Transformation|GetRelativeTransform (Variables|Default|GetVR_door_A_VR_door_R)))) false false)
      (Transformation|SetRelativeTransform (Variables|Default|GetVR_door_A_VR_door_L) (Math|Transform|MakeTransform (Math|Vector|MakeVector (.x _door_l) (.y _door_l) (.z _door_l)) (Math|Rotator|MakeRotator 0.0 0.0 (Math|Float|Lerp 0.0 -9e+01 _新規track_1)) (.scale (Transformation|GetRelativeTransform (Variables|Default|GetVR_door_A_VR_door_L)))) false false))))

(event EventBeginPlay
  (bind _returnvalue (Actor|GetActorOfClass "/Script/GhostBurster.VRPlayerCharacter"))
  (Variables|Default|Setplayer _returnvalue)
  (Variables|Default|Setdoor_R (.location (Transformation|GetRelativeTransform (Variables|Default|GetVR_door_A_VR_door_R))))
  (Variables|Default|Setdoor_L (.location (Transformation|GetRelativeTransform (Variables|Default|GetVR_door_A_VR_door_L)))))

(fn ConstructionScript)
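; BP_Lamp_ is a flickering lamp whose light starts hidden and repeatedly switches on and off.
; Tick counts down the off time, shows the light, then a latent Delay holds it on before hiding it.
; The parity of a counter alternates the timings, so a short flash after a random dark gap is followed by a brief gap and a randomly timed lit period.
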(event EventBeginPlay
  (Variables|Default|SetTimer_OffToOn 2.5)
  (Variables|Default|SetTimer_OnToOff 0.2)
  (Rendering|SetVisibility (Variables|Default|GetLight) false false))

(event EventTick
  (params (DeltaSeconds :type Float%20%28single-precision%29))
  ;[1 1 1] カウントダウン
  (bind _output_get (Variables|Default|SetTimer_OffToOn (- (Variables|Default|GetTimer_OffToOn) DeltaSeconds)))
  ;[1 1 1] ライトを点ける
  (if (<= _output_get 0.0)
    (Rendering|SetVisibility (Variables|Default|GetLight) true false)
    (Utilities|FlowControl|Delay (Variables|Default|GetTimer_OnToOff)) ; 消すまでの時間
    ;[1 1 1] ライトを消す
    (Rendering|SetVisibility (Variables|Default|GetLight) false false)
    (bind _result (Math|Integer|IncrementInt (Variables|Default|GetCount))
      (:%20%20
        (if (== (Math|Integer|%(Integer) _result 2) 0)
          ;[1 1 1] 次に電気が点く回数が奇数
          (Variables|Default|SetTimer_OffToOn (Math|Random|RandomFloatinRange (Variables|Default|GetOffToOn_Min) (Variables|Default|GetOffToOn_Max)))
          (Variables|Default|SetTimer_OnToOff 0.2)
          (else
            ;[1 1 1] 次に電気が点く回数が偶数
            (Variables|Default|SetTimer_OffToOn 0.2)
            (Variables|Default|SetTimer_OnToOff (Math|Random|RandomFloatinRange (Variables|Default|GetOnToOff_Min) (Variables|Default|GetOnToOff_Max)))))))))

(fn ConstructionScript)
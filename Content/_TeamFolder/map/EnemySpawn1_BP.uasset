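; EnemySpawn1_BP is a trigger actor that halts the player's spline movement and starts an enemy encounter.
; On BeginPlay it caches the BP_PlayerSpline and VRPlayerCharacter; when the player's collision overlaps its Box, it stops the spline and spawns a GreenEnemy and a NormalEnemy at hard-coded locations.
; EnemyDeadFunction decrements and prints the enemy count, but its zero branch is empty, with the next-stage, resume-movement and self-destroy calls left disconnected.
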(event OnComponentBeginOverlap(Box)
  (params (OverlappedComponent :type Primitive%20Component%20Object%20Reference) (OtherActor :type Actor%20Object%20Reference) (OtherComp :type Primitive%20Component%20Object%20Reference) (OtherBodyIndex :type Integer) (bFromSweep :type Boolean) (SweepResult :type Hit%20Result%20Structure%20%28by%20ref%29))
  (if (== OtherComp (Variables|/Script/GhostBurster.VRPlayerCharacter|GetPlayerCollision (Variables|Default|GetPlayer)))
    ;[1 1 1] プレイヤーの移動を止める
    (Class|PlayerSplinePath|StopMovement (Variables|Default|GetSpline))
    ;[1 1 1] 敵の生成
    (Variables|Default|SetEnemyCount 0)
    (Game|SpawnActorfromClass "/Script/GhostBurster.GreenEnemy" (Math|Conversions|ToTransform(Vector) "4000.000000,-450.000000,200.000000") "Undefined" "MultiplyWithRoot" 0 0)
    (Variables|Default|SetEnemyCount (+ (Variables|Default|GetEnemyCount) 1))
    (Game|SpawnActorfromClass "/Script/GhostBurster.NormalEnemy" (Math|Conversions|ToTransform(Vector) "4000.000000,500.000000,300.000000") "Undefined" "MultiplyWithRoot" 0 0)
    (Variables|Default|SetEnemyCount (+ (Variables|Default|GetEnemyCount) 1))))

(event EventBeginPlay
  (bind _returnvalue (Actor|GetActorOfClass "/Game/_TeamFolder/Player/Blueprint/BP_PlayerSpline.BP_PlayerSpline_C"))
  (Variables|Default|SetSpline _returnvalue)
  (bind _returnvalue_2 (Actor|GetActorOfClass "/Script/GhostBurster.VRPlayerCharacter"))
  (Variables|Default|SetPlayer _returnvalue_2))

(event Collision|EventActorBeginOverlap
  (params (OtherActor :type Actor%20Object%20Reference)))

(event EventTick
  (params (DeltaSeconds :type Float%20%28single-precision%29)))

(fn ConstructionScript)

(fn EnemyDeadFunction
  (Variables|Default|SetEnemyCount (- (Variables|Default|GetEnemyCount) 1))
  (Development|PrintString (Utilities|String|Append "Call" (Utilities|String|ToString(Integer) (Variables|Default|GetEnemyCount))) true true "(R=1.000000,G=0.000000,B=0.928275,A=1.000000)")
  (if (== (Variables|Default|GetEnemyCount) 0)
    _))
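; Trigger-box enemy spawner for a VR game in which the player moves along a spline path.
; When the player's collision enters the box, it stops spline movement, passes itself to the player and calls ItemControlPlay.
; It then uses the player's stage number as the wave for SpawnEnemiesForWave, whose body is not shown here.
; An unconnected stage switch with hardcoded enemy and boss spawn positions remains in the graph but never runs.
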(event OnComponentBeginOverlap(Box)
  (params (OverlappedComponent :type Primitive%20Component%20Object%20Reference) (OtherActor :type Actor%20Object%20Reference) (OtherComp :type Primitive%20Component%20Object%20Reference) (OtherBodyIndex :type Integer) (bFromSweep :type Boolean) (SweepResult :type Hit%20Result%20Structure%20%28by%20ref%29))
  (bind _player (Variables|Default|GetPlayer))
  (if (== OtherComp (Variables|/Script/GhostBurster.VRPlayerCharacter|GetPlayerCollision (Variables|Default|Getplayer)))
    ;[1 1 1] プレイヤーを止める
    (Class|PlayerSplinePath|StopMovement (Variables|Default|GetSpline))
    ;[1 1 1] プレイヤーにスポナーをセット
    (Class|EnemySpawner|SendSelftoPlayer)
    (Class|VRPlayerCharacter|ItemControlPlay _player)
    ;[1 1 1] Waveに合わせてEnemyをスポーンさせる
    (bind _returnvalue (Class|VRPlayerCharacter|GetStageNumber _player))
    (bind _output_get (Variables|Default|SetWave _returnvalue))
    (Class|EnemySpawner|SpawnEnemiesforWave _output_get)))

(event EventBeginPlay
  (bind _returnvalue (Actor|GetActorOfClass "/Script/GhostBurster.VRPlayerCharacter"))
  (Variables|Default|Setplayer _returnvalue)
  (bind _returnvalue_2 (Actor|GetActorOfClass "/Script/GhostBurster.PlayerSplinePath"))
  (Variables|Default|SetSpline _returnvalue_2))

(fn ConstructionScript)
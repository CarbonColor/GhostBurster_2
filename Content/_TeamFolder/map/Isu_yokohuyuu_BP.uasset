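; Blueprint for a chair (Isu) that floats sideways, moving its VRIsu component from the start of play.
; BeginPlay caches the component's relative location and starts the floating event, which plays a timeline.
; Three timeline tracks separately drive lerps for a sideways Y offset, a vertical rise and a yaw turn.
; Each update rewrites the relative transform, keeping scale but leaving X, pitch and roll unwired.
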(event Custom|isu_yokofloating
  (bind _isu_transform (Variables|Default|Getisu_transform))
  (bind (_direction _新規track_0 _新規track_1 _新規track_2) (Timeline|タイムライン_0 Play)
    (:Update
      (Transformation|SetRelativeTransform (Variables|Default|GetVR_isu) (Math|Transform|MakeTransform (Math|Vector|MakeVector 0.0 (Math|Float|Lerp (.y _isu_transform) (+ (.y _isu_transform) 8e+01) _新規track_2) (Math|Float|Lerp (.z _isu_transform) (+ (.z _isu_transform) 4e+01) _新規track_0)) (Math|Rotator|MakeRotator 0.0 0.0 (Math|Float|Lerp 0.0 75.0 _新規track_1)) (.scale (Transformation|GetRelativeTransform (Variables|Default|GetVR_isu)))) false false))))

(event EventBeginPlay
  (Variables|Default|Setisu_transform (.location (Transformation|GetRelativeTransform (Variables|Default|GetVR_isu))))
  (CallFunction|IsuYokofloating))

(event Collision|EventActorBeginOverlap
  (params (OtherActor :type Actor%20Object%20Reference)))

(event EventTick
  (params (DeltaSeconds :type Float%20%28single-precision%29)))

(fn ConstructionScript)
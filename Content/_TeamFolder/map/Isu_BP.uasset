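; Chair Blueprint (Isu_BP) that makes its VRIsu component float upward while turning around.
; BeginPlay caches the component's relative location as the starting point.
; The custom float event (椅子浮遊) plays a two-track timeline that lerps relative height above that start and yaw through a half turn, keeping the current scale.
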(event Custom|椅子浮遊
  (bind _isu_transform (Variables|Default|Getisu_transform))
  (bind (_direction _新規track_0 _新規track_1) (Timeline|タイムライン_0 Play)
    (:Update
      (Transformation|SetRelativeTransform (Variables|Default|GetVR_isu) (Math|Transform|MakeTransform (Math|Vector|MakeVector 0.0 0.0 (Math|Float|Lerp (.z _isu_transform) (+ (.z _isu_transform) 5e+01) _新規track_0)) (Math|Rotator|MakeRotator 0.0 0.0 (Math|Float|Lerp 0.0 1.8e+02 _新規track_1)) (.scale (Transformation|GetRelativeTransform (Variables|Default|GetVR_isu)))) false false))))

(event EventBeginPlay
  (Variables|Default|Setisu_transform (.location (Transformation|GetRelativeTransform (Variables|Default|GetVR_isu)))))

(event Collision|EventActorBeginOverlap
  (params (OtherActor :type Actor%20Object%20Reference)))

(event EventTick
  (params (DeltaSeconds :type Float%20%28single-precision%29)))

(fn ConstructionScript)